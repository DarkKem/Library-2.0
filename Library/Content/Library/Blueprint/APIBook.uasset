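; Actor that fills the game's libraries with books fetched from a web API.
; On BeginPlay it pools spawn points from every Library actor, then sends a VaRest GET request to a mockapi.io endpoint.
; The response handler spawns one Book per JSON entry at the next pooled point, removing that point, and sets its title, author and pages.
; The failure handler is empty.
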(event Custom|Rsponse%20book
  (params (Request :type Va%20Rest%20Request%20JSON%20Object%20Reference))
  (for _array_element (Class|VaRestJsonValue|AsArray (Class|VaRestRequestJSON|GetResponseValue Request))
    (bind _returnvalue (Class|VaRestJsonValue|AsObject _array_element))
    (bind _spawn (CallFunction|GetSpawnPoint))
    (bind _returnvalue_2 (Game|SpawnActorfromClass "/Game/Library/Blueprint/Book.Book_C" _spawn "Undefined" 0 0))
    (Variables|/Game/Library/Blueprint/Book.Book_C|Settitle _returnvalue_2 (Class|VaRestJsonObject|GetStringField _returnvalue "title"))
    (Variables|/Game/Library/Blueprint/Book.Book_C|Setauteur _returnvalue_2 (Class|VaRestJsonObject|GetStringField _returnvalue "auteur"))
    (Variables|/Game/Library/Blueprint/Book.Book_C|Setpage _returnvalue_2 (Class|VaRestJsonObject|GetStringArrayField _returnvalue "page"))
    (Default|SetValue _returnvalue_2)))

(event Custom|Response%20error%20book
  (params (Request :type Va%20Rest%20Request%20JSON%20Object%20Reference)))

(event Collision|EventActorBeginOverlap
  (params (OtherActor :type Actor%20Object%20Reference)))

(event EventTick
  (params (DeltaSeconds :type Float%20%28single-precision%29)))

(event EventBeginPlay
  (CallFunction|SetSpawnPoint)
  (bind _returnvalue (Class|VaRestSubsystem|ConstructVaRestRequestExt (|VaRestSubsystem) "GET" "x_www_form_urlencoded_body"))
  (bind _output_get (Variables|Default|SetJson%20request _returnvalue))
  (EventDispatchers|BindEventtoOnRequestComplete _output_get (delegate Custom|Rsponse%20book))
  (EventDispatchers|BindEventtoOnRequestFail _output_get (delegate Custom|Response%20error%20book))
  (Class|VaRestRequestJSON|ProcessURL (Variables|Default|GetJson%20request) "https://62c828578c90491c2cb00efa.mockapi.io/book"))

(fn ConstructionScript)

(fn SetSpawnPoint
  (bind _outactors (Actor|GetAllActorsOfClass "/Game/Library/library.library_C"))
  (for _array_element _outactors
    (bind _aslibrary (Utilities|Casting|CastTolibrary _array_element))
    (bind _spawnlist (Default|GetSpawnPointList _aslibrary))
    (Utilities|Array|AppendArray (Variables|Default|GetSpawnPoint) _spawnlist)))

(fn GetSpawnPoint
  (if (>= (Utilities|Array|Length (Variables|Default|GetSpawnPoint)) 1)
    (LocalVariables|Setpoint (Utilities|Array|Get(acopy) (Variables|Default|GetSpawnPoint)))
    (Utilities|Array|RemoveIndex (Variables|Default|GetSpawnPoint))
    (return (LocalVariables|Getpoint))))