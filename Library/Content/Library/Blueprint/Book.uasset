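; Book actor for the library, showing a title, an author and page text on a grabbable object.
; SetValue writes the title and author strings to their text components and puts the first Page entry into a TextWidget hosted by the PageWidget component.
; Grabbing it through its GrabComponent turns on physics simulation for the Cube mesh.
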(event OnGrabbed(GrabComponent)
  (Physics|SetSimulatePhysics (Variables|Default|GetCube) true))

(event EventBeginPlay)

(event Collision|EventActorBeginOverlap
  (params (OtherActor :type Actor%20Object%20Reference)))

(event EventTick
  (params (DeltaSeconds :type Float%20%28single-precision%29)))

(fn ConstructionScript)

(fn SetValue
  (Rendering|Components|TextRender|SetText (Variables|Default|GetTitleComp) (Utilities|Text|ToText(String) (Variables|Default|Gettitle)))
  (Rendering|Components|TextRender|SetText (Variables|Default|GetAuteurComp) (Utilities|Text|ToText(String) (Variables|Default|Getauteur)))
  (bind _astext_widget (Utilities|Casting|CastToTextWidget (UserInterface|GetWidget (Variables|Default|GetPageWidget))))
  (Variables|/Game/Library/Widget/TextWidget.TextWidget_C|SetText _astext_widget (Utilities|Text|ToText(String) (Utilities|Array|Get(acopy) (Variables|Default|Getpage)))))