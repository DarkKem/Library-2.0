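; Blue cat character Blueprint that roams, approaches the player or rests, driven by state flags and an energy level.
; DecideNextAction picks AI MoveTo roaming or a faster approach, re-deciding after each successful move and a random delay.
; A self-recalling one-second drain loop sets IsTried at zero energy, triggering energy regain and a timed lie-down.
; Rest plays raw animations, then restores the Animation Blueprint and restarts draining.
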(event Custom|Decide%20Next%20Action
  (params (Skip%20Delay? :type Boolean))
  ;[1 1 1] Decide next action
  (if Skip%20Delay?
    _
    (else
      (Utilities|FlowControl|Delay (Math|Conversions|ToFloat(Integer) (Math|Random|RandomIntegerinRange 1 5)))))
  (if (Variables|Default|GetIsTried)
    (CallFunction|RegainEnergy)
    (CallFunction|Rest)
    (elif (Variables|Default|GetIsIritated)
      (CallFunction|RandomRoam :!label _label)
      (elif (Variables|Default|GetWantAttention)
        (goto _label)
        (elif (Variables|Default|GetComeCloser)
          (CallFunction|ComeCloser)
          (else
            (goto _label)))))))

(event Custom|Come%20closer
  ;[1 1 1] Come closer
  (Variables|/Script/Engine.CharacterMovementComponent|SetMaxWalkSpeed (Variables|Character|GetCharacterMovement) 3e+02)
  (AI|AIMoveTo self (Transformation|GetActorLocation (Game|Player|GetPlayerPawn 0)) 0 5.0 false
    (:OnSuccess
      (CallFunction|DecideNextAction false))))

(event Custom|Random%20Roam
  ;[1 1 1] Random roam
  (Variables|/Script/Engine.CharacterMovementComponent|SetMaxWalkSpeed (Variables|Character|GetCharacterMovement) 1.5e+02)
  (AI|AIMoveTo self (.RandomLocation (AI|Navigation|GetRandomReachablePointinRadius (Transformation|GetActorLocation) 1.5e+03 0 0)) 0 5.0 false
    (:OnSuccess
      (CallFunction|DecideNextAction false))))

(event Custom|Rest
  ;[1 1 1] Rest
  (Components|Movement|StopMovementImmediately (Variables|Character|GetCharacterMovement))
  (CallFunction|PlayAnimation false "/Game/LowPoly_Cat/Animations/Anim_Cat_Lie_start.Anim_Cat_Lie_start")
  (Utilities|FlowControl|Delay 0.24)
  (CallFunction|PlayAnimation true "/Game/LowPoly_Cat/Animations/Anim_Cat_Lie_loop.Anim_Cat_Lie_loop")
  (Utilities|FlowControl|Delay (Math|Conversions|ToFloat(Integer) (Math|Random|RandomIntegerinRange 0 60)))
  (CallFunction|PlayAnimation false "/Game/LowPoly_Cat/Animations/Anim_Cat_Lie_end.Anim_Cat_Lie_end")
  (Utilities|FlowControl|Delay 0.24)
  (CallFunction|StopAnimation)
  (Variables|Default|SetIsTried false)
  (CallFunction|DecideNextAction false)
  (CallFunction|DrainEnergy))

(event Custom|Drain%20Energy
  ;[1 1 1] Drain energy
  (if (not (Variables|Default|GetIsTried))
    (bind _output_get (Variables|Energy|SetEnergy (Math|Integer|Clamp(Integer) (- (Variables|Energy|GetEnergy) (Variables|Energy|GetEnergy%20Drain)) 0 (Variables|Energy|GetMax%20Energy))))
    (if (== _output_get 0)
      (Variables|Default|SetIsTried true)
      (CallFunction|DecideNextAction false)
      (else
        (Utilities|FlowControl|Delay 1.0)
        (CallFunction|DrainEnergy)))))

(event Custom|Regain%20Energy
  ;[1 1 1] Regain energy
  (if (Variables|Default|GetIsTried)
    (bind _output_get (Variables|Energy|SetEnergy (Math|Integer|Clamp(Integer) (+ (Variables|Energy|GetEnergy) (Variables|Energy|GetEnergy%20Gain)) 0 (Variables|Energy|GetMax%20Energy))))
    (if (not (== _output_get (Variables|Energy|GetMax%20Energy)))
      (Utilities|FlowControl|Delay 1.0)
      (CallFunction|RegainEnergy))))

(event EventBeginPlay
  (CallFunction|DecideNextAction false)
  (CallFunction|DrainEnergy))

(fn ConstructionScript)

(fn PlayAnimation
  (params (Should%20Loop%20? :type Boolean) (Animation :type Animation%20Asset%20Object%20Reference))
  (Components|Animation|PlayAnimation (Variables|Character|GetMesh) Animation Should%20Loop%20?))

(fn StopAnimation
  (bind _mesh (Variables|Character|GetMesh))
  (Components|Animation|SetAnimationMode _mesh "AnimationBlueprint")
  (Class|SkeletalMeshComponent|SetAnimClass _mesh "/Game/Library/Cat/AnimationCatBP.AnimationCatBP_C"))